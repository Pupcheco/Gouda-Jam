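; BP_EvidenceDesk is an evidence drop-off that decides when the player has won by collecting three true pieces of evidence.
; Its detection box records matching overlapping actors once each and clears the game mode's NewestEvidence.
; Every Tick polls the collection: all three true items end the loop and set the game as won.
; A second check flags CheckEvidence on FirstPersonGameMode when a collection is partial.
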(event OnComponentBeginOverlap(Evidencedetectionbox)
  (params (OverlappedComponent :type Primitive%20Component%20Object%20Reference) (OtherActor :type Actor%20Object%20Reference) (OtherComp :type Primitive%20Component%20Object%20Reference) (OtherBodyIndex :type Integer) (bFromSweep :type Boolean) (SweepResult :type Hit%20Result%20Structure%20%28by%20ref%29))
  (Variables|Default|SetHit%20Actor OtherActor)
  (if (Math|Boolean|ORBoolean (== (Variables|Default|GetHit%20Actor) 0) (== (Variables|Default|GetHit%20Actor) 0) (== (Variables|Default|GetHit%20Actor) 0))
    (if (not (Utilities|Array|ContainsItem (Variables|Default|GetEvidence%20collected) (Variables|Default|GetHit%20Actor)))
      (Utilities|Array|AddUnique (Variables|Default|GetEvidence%20collected) (Variables|Default|GetHit%20Actor))
      (bind _asfirst_person_game_mode (Utilities|Casting|CastToFirstPersonGameMode (Game|GetGameMode)))
      (Variables|/Game/FirstPersonBP/Blueprints/FirstPersonGameMode.FirstPersonGameMode_C|Setnewest%20evidence _asfirst_person_game_mode 0))))

(event EventTick
  (params (DeltaSeconds :type Float%20%28single-precision%29))
  (bind _evidence_collected (Variables|Default|GetEvidence%20collected))
  (bind _evidence_collected_2 (Variables|Default|GetEvidence%20collected))
  (bind _evidence_collected_3 (Variables|Default|GetEvidence%20collected))
  (Utilities|FlowControl|Sequence
    (:then_0
      (if (Math|Boolean|ANDBoolean (Utilities|Array|ContainsItem _evidence_collected_2 (Variables|Default|GetTrue%20Evidence%201)) (Utilities|Array|ContainsItem _evidence_collected_2 (Variables|Default|GetTrue%20Evidence%202)) (Utilities|Array|ContainsItem _evidence_collected_2 (Variables|Default|GetTrue%20Evidence%203)))
        (bind _asfirst_person_game_mode (Utilities|Casting|CastToFirstPersonGameMode (Game|GetGameMode)))
        (Variables|/Game/FirstPersonBP/Blueprints/FirstPersonGameMode.FirstPersonGameMode_C|SetLoop? _asfirst_person_game_mode false)
        (Variables|/Game/FirstPersonBP/Blueprints/FirstPersonGameMode.FirstPersonGameMode_C|SetIs%20game%20won? _asfirst_person_game_mode true)))
    (:then_1
      (if (Math|Boolean|ORBoolean (Utilities|Array|ContainsItem _evidence_collected_3 0) (Utilities|Array|ContainsItem _evidence_collected_3 0) (Utilities|Array|ContainsItem _evidence_collected_3 0))
        (if (not (Math|Boolean|ANDBoolean (Utilities|Array|ContainsItem _evidence_collected 0) (Utilities|Array|ContainsItem _evidence_collected 0) (Utilities|Array|ContainsItem _evidence_collected 0)))
          (bind _asfirst_person_game_mode_2 (Utilities|Casting|CastToFirstPersonGameMode (Game|GetGameMode)))
          (Variables|/Game/FirstPersonBP/Blueprints/FirstPersonGameMode.FirstPersonGameMode_C|Setcheck%20evidence _asfirst_person_game_mode_2 true))))))

(event EventBeginPlay
  (bind _evidence (Variables|Default|GetEvidence))
  (Utilities|Array|Add _evidence (Variables|Default|GetTrue%20Evidence%201))
  (Utilities|Array|Add _evidence (Variables|Default|GetTrue%20Evidence%202))
  (Utilities|Array|Add _evidence (Variables|Default|GetTrue%20Evidence%203)))

(fn ConstructionScript)